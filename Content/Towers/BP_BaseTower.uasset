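; BP_BaseTower is a tower that automatically fires homing arrow projectiles at enemies within its sphere range.
; Sphere overlaps add and remove BP_BaseEnemy actors in EnemyArray.
; A looping timer, created on first entry, paused when the array empties and unpaused on later entries, spawns arrows at ArrowSpawner.
; Each arrow receives the tower's Damage and homes on the capsule of the first enemy in the array.
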(event `self.Sphere.OnComponentBeginOverlap`
  (params (OverlappedComponent :type "PrimitiveComponent Object Reference") (OtherActor :type "Actor Object Reference") (OtherComp :type "PrimitiveComponent Object Reference") (OtherBodyIndex :type Integer) (bFromSweep :type Boolean) (SweepResult :type "HitResult Structure (by ref)"))
  (bind _spawnprojectiletimerhandle (`self.SpawnProjectileTimerHandle`))
  ; Shoot
  (bind _asbp_base_enemy (cast `/Game/Enemies/BP_BaseEnemy` OtherActor))
  (`KismetArrayLibrary.Array_AddUnique` (`self.EnemyArray`) _asbp_base_enemy)
  (if (`KismetSystemLibrary.K2_IsValidTimerHandle` _spawnprojectiletimerhandle)
    (`KismetSystemLibrary.K2_UnPauseTimerHandle` _spawnprojectiletimerhandle)
    (else
      (bind _returnvalue (`KismetSystemLibrary.K2_SetTimerDelegate` (delegate `SpawnProjectile`) (`self.delayTime`) true))
      (set `self.SpawnProjectileTimerHandle` _returnvalue))))

(event `SpawnProjectile`
  ; Shoot
  (bind _returnvalue (`|SpawnActorFromClass` "/Game/Towers/ArrowProjectile.ArrowProjectile_C" (`SceneComponent.K2_GetComponentToWorld` (`self.ArrowSpawner`)) "Undefined" "MultiplyWithRoot" null (`self.Damage`) self))
  (set `ProjectileMovementComponent.HomingTargetComponent` (`Character.CapsuleComponent` (`|GetArrayItem` (`self.EnemyArray`))) (`/Game/Towers/ArrowProjectile.ProjectileMovement` _returnvalue)))

(event `self.Sphere.OnComponentEndOverlap`
  (params (OverlappedComponent :type "PrimitiveComponent Object Reference") (OtherActor :type "Actor Object Reference") (OtherComp :type "PrimitiveComponent Object Reference") (OtherBodyIndex :type Integer))
  (bind _enemyarray (`self.EnemyArray`))
  ; Shoot
  (bind _asbp_base_enemy (cast `/Game/Enemies/BP_BaseEnemy` OtherActor))
  (`KismetArrayLibrary.Array_RemoveItem` _enemyarray _asbp_base_enemy)
  (if (`KismetArrayLibrary.Array_IsEmpty` _enemyarray)
    (`KismetSystemLibrary.K2_PauseTimerHandle` (`self.SpawnProjectileTimerHandle`))))

(fn `UserConstructionScript`)