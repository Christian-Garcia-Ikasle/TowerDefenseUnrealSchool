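; Game mode for a tower defense game that tracks player life, points and living enemies, and decides victory or defeat.
; It creates the WBP_UI HUD and pushes life, points and level number to it as they change.
; Enemy deaths award points and trigger an end-of-level check, which shows level UI or declares victory once the final level is cleared.
; Victory and defeat only print a message and pause the game.
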(event `NewLevel`
  ; New Level Actions
  (set `self.LevelEnd` false))

(event `self.ReceiveBeginPlay`
  (bind _hud (`self.HUD`))
  ; Set WBP
  (add `self.LevelStart` (delegate `NewLevel`))
  (bind _returnvalue (`|CreateWidget` "/Game/WBP_UI.WBP_UI_C"))
  (bind _output_get (set `self.HUD` _returnvalue))
  (`/Game/WBP_UI.SetTextHP` _output_get (`self.LifePointsPlayer`))
  (`/Game/WBP_UI.SetTextPoints` _hud (`self.PointsPlayer`))
  (`KismetSystemLibrary.DelayUntilNextTick`)
  (`UserWidget.AddToViewport` _hud 0))

(event `GetDamagePlayer`
  (params (Damage :type "Float (double-precision)"))
  ; Player receive damage
  (bind _output_get (set `self.LifePointsPlayer` (- (`self.LifePointsPlayer`) Damage)))
  (`/Game/WBP_UI.SetTextHP` (`self.HUD`) _output_get)
  (if (<= _output_get 0.0)
    (`self.Defeat`)))

(event `EnemyDead`
  (params (Points :type "Float (double-precision)") (Enemy :type "/Game/Enemies/BP_BaseEnemy Object Reference (by ref)"))
  ; Player Receive Points
  (bind _output_get (set `self.PointsPlayer` (+ (`self.PointsPlayer`) Points)))
  (`/Game/WBP_UI.SetTextPoints` (`self.HUD`) _output_get)
  (`self.EmemyDown` Enemy)
  (`self.EndLevel`))

(event `EndLevel`
  ; EndLevelCheck
  (if (and (`KismetArrayLibrary.Array_IsEmpty` (`self.EnemiesAlive`)) (`self.LevelEnd`))
    (if (and (`self.LevelEnd`) (`self.GameEnd`))
      (`self.Victory`)
      (else
        (`/Game/WBP_UI.SetUIVisible` (`self.HUD`))))))

(event `GetLevelNum`
  (params (LevelNum :type Integer))
  ; Get Level Number
  (`/Game/WBP_UI.SetTextLevel` (`self.HUD`) LevelNum))

(fn `Defeat`
  (`KismetSystemLibrary.PrintString` "Game Over")
  (`GameplayStatics.SetGamePaused` true))

(fn `EmemyDown`
  (params (Enemy :type "/Game/Enemies/BP_BaseEnemy Object Reference (by ref)"))
  (`KismetArrayLibrary.Array_RemoveItem` (`self.EnemiesAlive`) Enemy))

(fn `EnemySpawn`
  (params (Enemy :type "/Game/Enemies/BP_BaseEnemy Object Reference (by ref)"))
  (`KismetArrayLibrary.Array_Add` (`self.EnemiesAlive`) Enemy))

(fn `UserConstructionScript`)

(fn `Victory`
  (`KismetSystemLibrary.PrintString` "You Win")
  (`GameplayStatics.SetGamePaused` true))