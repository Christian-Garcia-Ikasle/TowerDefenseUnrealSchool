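; Tower-defense enemy spawner that spawns enemies at its own location, driven by an EnemyWave array.
; BeginPlay either calls Victory on GM_TowerDefense if the wave counter exceeds the array, or enters a DoN to wait that wave's WaveTimer.
; A second DoN re-enters itself to spawn timed enemies up to the wave count, then resets.
; Each enemy receives a billboard-marked Destination and its start location.
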(event `self.ReceiveBeginPlay`
  (bind _enemywave (`self.EnemyWave`))
  (bind _returnvalue (`KismetArrayLibrary.Array_Length` _enemywave))
  ; Spawn enemies
  (if (> (stale _counter) _returnvalue)
    (bind _asgm_tower_defense (cast `/Game/GM_TowerDefense` (`GameplayStatics.GetGameMode`)))
    (`/Game/GM_TowerDefense.Victory` _asgm_tower_defense)
    (else
      (bind _counter (`/Engine/EditorBlueprintResources/StandardMacros.Do N` _returnvalue)
        (:`Exit`
          (bind (_numenemies _enemytype _spawntimer _wavetimer) (break `/Game/S_EnemyWave` (`|GetArrayItem` _enemywave (- _counter 1))))
          (`KismetSystemLibrary.Delay` _wavetimer)
          (bind _counter_2 (`/Engine/EditorBlueprintResources/StandardMacros.Do N` _numenemies :!label _label)
            (:`Exit`
              (`KismetSystemLibrary.Delay` _spawntimer)
              (bind _returnvalue_2 (`|SpawnActorFromClass` _enemytype (`self.GetTransform`) "AlwaysSpawn" "MultiplyWithRoot" null null))
              (set `/Game/BP_BaseEnemy.Destination` (`SceneComponent.K2_GetComponentLocation` (`self.DestinationBillboard`)) _returnvalue_2)
              (set `/Game/BP_BaseEnemy.StartLoc` (`SceneComponent.K2_GetComponentLocation` (`self.DefaultSceneRoot`)) _returnvalue_2)
              (if (>= _counter_2 _numenemies)
                (`|ExecutionSequence`
                  (:`then_0`
                    (goto _label :!via `Reset`)))
                (else
                  (goto _label))))))))))

(fn `UserConstructionScript`)