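; Tower defense enemy spawner that runs per-level waves from LevelData and gives each enemy a start point and billboard destination.
; The game mode's level start event triggers RoundManager, which loads the level's waves and begins the current one.
; A looping timer with per-wave delays spawns enemies up to the wave count, reporting each to GM_TowerDefense.
; Completed spawning advances the wave or level, setting the game mode's LevelEnd and GameEnd flags.
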(event `self.ReceiveBeginPlay`
  ; Spawner
  (bind _asgm_tower_defense (cast `/Game/GM_TowerDefense` (`GameplayStatics.GetGameMode`)))
  (bind _output_get (set `self.As GM Tower Defense` _asgm_tower_defense))
  (add `/Game/GM_TowerDefense.LevelStart` _output_get (delegate `RoundManager`)))

(event `NextWave`
  ; Spawner
  (set `self.WaveData` (`|GetArrayItem` (`self.EnemyWave`) (`self.WaveID`)) :!label _label)
  (bind _returnvalue (`KismetSystemLibrary.K2_SetTimerDelegate` (delegate `SpawnEnemies`) (`self.GetCurrentWaveSpawnDelay`) true false (`self.GetCurrentWaveDelay`)))
  (set `self.SpawnTimerHandle` _returnvalue))

(event `RoundManager`
  (bind _output_enemywave (break `/Game/Enemies/S_Level` (`|GetArrayItem` (`self.LevelData`) (`self.Level ID`))))
  ; Spawner
  (if (< (`self.Level ID`) (`KismetArrayLibrary.Array_Length` (`self.LevelData`)))
    (set `self.EnemyWave` _output_enemywave)
    (if (`KismetArrayLibrary.Array_IsValidIndex` (`self.EnemyWave`) (`self.WaveID`))
      (goto _label)
      (else
        (`self.Wave&LevelCheck`)))))

(event `SpawnEnemies`
  ; Spawner
  (if (>= (`self.EnemyCount`) (`self.GetCurrentEnemyNumber`))
    (`self.Wave&LevelCheck`)
    (else
      (bind _returnvalue (`|SpawnActorFromClass` (`self.GetCurrentEnemyClass`) (`self.GetTransform`) "AdjustIfPossibleButAlwaysSpawn" "MultiplyWithRoot" null null))
      (set `/Game/Enemies/BP_BaseEnemy.Destination` (`SceneComponent.K2_GetComponentLocation` (`self.DestinationBillboard`)) _returnvalue)
      (set `/Game/Enemies/BP_BaseEnemy.StartLoc` (`SceneComponent.K2_GetComponentLocation` (`self.DefaultSceneRoot`)) _returnvalue)
      (`/Engine/EditorBlueprintResources/StandardMacros.IncrementInt` (`self.EnemyCount`)
        (:`  `
          (`/Game/GM_TowerDefense.EnemySpawn` (`self.As GM Tower Defense`) _returnvalue))))))

(fn `GetCurrentEnemyClass`
  (returns (`Wave Data Enemy Type` :type "/Game/Enemies/BP_BaseEnemy Class Reference"))
  (bind (_wavedata_numenemies _wavedata_enemytype) (break `/Game/Enemies/S_EnemyWave` (`self.WaveData`)))
  (return _wavedata_enemytype))

(fn `GetCurrentEnemyNumber`
  (returns (EnemyNumber :type Integer))
  (bind _wavedata_numenemies (break `/Game/Enemies/S_EnemyWave` (`self.WaveData`)))
  (return _wavedata_numenemies))

(fn `GetCurrentWaveDelay`
  (returns (WaveDelay :type "Float (double-precision)"))
  (bind (_wavedata_numenemies _wavedata_enemytype _wavedata_spawndelay _wavedata_wavedelay) (break `/Game/Enemies/S_EnemyWave` (`self.WaveData`)))
  (return _wavedata_wavedelay))

(fn `GetCurrentWaveSpawnDelay`
  (returns (SpawnDelay :type "Float (double-precision)"))
  (bind (_wavedata_numenemies _wavedata_enemytype _wavedata_spawndelay) (break `/Game/Enemies/S_EnemyWave` (`self.WaveData`)))
  (return _wavedata_spawndelay))

(fn `UserConstructionScript`)

(fn `Wave&LevelCheck`
  (set `self.EnemyCount` 0)
  (bind _result (`/Engine/EditorBlueprintResources/StandardMacros.IncrementInt` (`self.WaveID`))
    (:`  `
      (`KismetSystemLibrary.K2_ClearAndInvalidateTimerHandle` (`self.SpawnTimerHandle`))
      (if (`KismetArrayLibrary.Array_IsValidIndex` (`self.EnemyWave`) _result)
        (`self.NextWave`)
        (else
          (`/Engine/EditorBlueprintResources/StandardMacros.IncrementInt` (`self.Level ID`)
            (:`  `
              (bind _asgm_tower_defense (cast `/Game/GM_TowerDefense` (`GameplayStatics.GetGameMode`)))
              (bind _output_get (set `self.As GM Tower Defense` _asgm_tower_defense))
              (`/Game/GM_TowerDefense.GetLevelNum` _output_get (`self.Level ID`))
              (set `self.WaveID` 0)
              (set `/Game/GM_TowerDefense.LevelEnd` true (`self.As GM Tower Defense`))
              (if (not (`KismetArrayLibrary.Array_IsValidIndex` (`self.LevelData`) (`self.Level ID`)))
                (set `/Game/GM_TowerDefense.GameEnd` true (`self.As GM Tower Defense`))))))))))