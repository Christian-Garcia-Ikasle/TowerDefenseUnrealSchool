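; Base enemy for a tower defense game that walks to a goal, takes damage and can hurt the player.
; On possession it caches its AIC_Enemy controller and, a tick later, orders it to move to Destination.
; Any damage destroys the damage causer and lowers LifePoints; at zero it reports reward points to GM_TowerDefense and destroys itself.
; DealDamageToPlayer passes its damage value to the game mode.
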(event `self.ReceivePossessed`
  (params (NewController :type "Controller Object Reference"))
  ; Move to goal
  (bind _asaic_enemy (cast `/Game/Enemies/AIC_Enemy` NewController))
  (set `self.As AIC Enemy` _asaic_enemy)
  (`KismetSystemLibrary.DelayUntilNextTick`)
  (`/Game/Enemies/AIC_Enemy.MoveToGoalLocation` (`self.As AIC Enemy`) (`self.Destination`)))

(event `self.ReceiveAnyDamage`
  (params (Damage :type "Float (single-precision)") (DamageType :type "DamageType Object Reference") (InstigatedBy :type "Controller Object Reference") (DamageCauser :type "Actor Object Reference"))
  ; Receive Damage
  (`self.K2_DestroyActor` DamageCauser)
  (bind _output_get (set `self.LifePoints` (- (`self.LifePoints`) Damage)))
  (if (<= _output_get 0.0)
    ; Generate Points
    (bind _asgm_tower_defense (cast `/Game/GM_TowerDefense` (`GameplayStatics.GetGameMode`)))
    (`/Game/GM_TowerDefense.EnemyDead` _asgm_tower_defense (`self.RewardPoints`) self)
    (`self.K2_DestroyActor`)))

(fn `DealDamageToPlayer`
  (bind _asgm_tower_defense (cast `/Game/GM_TowerDefense` (`GameplayStatics.GetGameMode`)))
  (`/Game/GM_TowerDefense.GetDamagePlayer` _asgm_tower_defense (`self.DamageToPlayer`)))

(fn `UserConstructionScript`)