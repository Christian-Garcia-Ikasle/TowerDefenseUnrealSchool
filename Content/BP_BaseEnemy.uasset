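; Base enemy for a tower defense game that travels to a goal, takes damage and rewards the player on death.
; On possession it waits one tick, then has its AIC_Enemy controller move it to Destination.
; Any damage destroys the damage causer and lowers LifePoints; at zero the enemy destroys itself and adds money in GM_TowerDefense.
; DealDamageToPlayer decrements the player's life in that game mode, but is not called here.
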(event `self.ReceivePossessed`
  (params (NewController :type "Controller Object Reference"))
  ; Move to goal
  (bind _asaic_enemy (cast `/Game/AIC_Enemy` NewController))
  (set `self.As AIC Enemy` _asaic_enemy)
  (`KismetSystemLibrary.DelayUntilNextTick`)
  (`/Game/AIC_Enemy.MoveToGoalLocation` (`self.As AIC Enemy`) (`self.Destination`)))

(event `self.ReceiveAnyDamage`
  (params (Damage :type "Float (single-precision)") (DamageType :type "DamageType Object Reference") (InstigatedBy :type "Controller Object Reference") (DamageCauser :type "Actor Object Reference"))
  ; Receive Damage
  (`self.K2_DestroyActor` DamageCauser)
  (bind _output_get (set `self.LifePoints` (- (`self.LifePoints`) Damage)))
  (if (<= _output_get 0.0)
    (`self.K2_DestroyActor`)
    ; Generate Money
    (bind _asgm_tower_defense (cast `/Game/GM_TowerDefense` (`GameplayStatics.GetGameMode`)))
    (set `/Game/GM_TowerDefense.MoneyPlayer` (+ (`/Game/GM_TowerDefense.MoneyPlayer` _asgm_tower_defense) 2.0) _asgm_tower_defense)))

(fn `DealDamageToPlayer`
  (bind _asgm_tower_defense (cast `/Game/GM_TowerDefense` (`GameplayStatics.GetGameMode`)))
  (bind _result (`/Engine/EditorBlueprintResources/StandardMacros.DecrementFloat` (`/Game/GM_TowerDefense.LifePointsPlayer` _asgm_tower_defense))
    (:`  `
      (set `/Game/GM_TowerDefense.LifePointsPlayer` _result _asgm_tower_defense))))

(fn `UserConstructionScript`)