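; Test door actor that swings open when a BP_TopDownCharacter enters its Box trigger and back when it leaves.
; Begin and end overlap each start a looping 0.01-second timer that steps a shared Percentage up or down, lerping the Door's relative yaw across 90 degrees.
; Each timer pauses itself at its limit, but neither overlap stops the opposite timer, so both can run at once.
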(event `EventOpenUp`
  (bind _percentage (`self.Percentage`))
  (if (>= _percentage 1.0)
    (`KismetSystemLibrary.K2_PauseTimerHandle` (`self.Move Timer up`))
    (else
      (set `self.Percentage` (+ _percentage (`self.IncrementValue`)))
      (`SceneComponent.K2_SetRelativeRotation` (`self.Door`) (`KismetMathLibrary.MakeRotator` 0.0 0.0 (`KismetMathLibrary.Lerp` -90.0 0.0 _percentage)) false false))))

(event `self.Box.OnComponentBeginOverlap`
  (params (OverlappedComponent :type "PrimitiveComponent Object Reference") (OtherActor :type "Actor Object Reference") (OtherComp :type "PrimitiveComponent Object Reference") (OtherBodyIndex :type Integer) (bFromSweep :type Boolean) (SweepResult :type "HitResult Structure (by ref)"))
  (cast `/Game/TopDown/Blueprints/BP_TopDownCharacter` OtherActor)
  (bind _returnvalue (`KismetSystemLibrary.K2_SetTimerDelegate` (delegate `EventOpenUp`) 0.01 true))
  (set `self.Move Timer up` _returnvalue))

(event `self.Box.OnComponentEndOverlap`
  (params (OverlappedComponent :type "PrimitiveComponent Object Reference") (OtherActor :type "Actor Object Reference") (OtherComp :type "PrimitiveComponent Object Reference") (OtherBodyIndex :type Integer))
  (cast `/Game/TopDown/Blueprints/BP_TopDownCharacter` OtherActor)
  (bind _returnvalue (`KismetSystemLibrary.K2_SetTimerDelegate` (delegate `CustomEvent`) 0.01 true))
  (set `self.Move Timer down` _returnvalue))

(event `CustomEvent`
  (bind _percentage (`self.Percentage`))
  (if (<= _percentage 0.0)
    (`KismetSystemLibrary.K2_PauseTimerHandle` (`self.Move Timer down`))
    (else
      (set `self.Percentage` (- _percentage (`self.IncrementValue`)))
      (`SceneComponent.K2_SetRelativeRotation` (`self.Door`) (`KismetMathLibrary.MakeRotator` 0.0 0.0 (`KismetMathLibrary.Lerp` -90.0 0.0 _percentage)) false false))))

(fn `UserConstructionScript`)